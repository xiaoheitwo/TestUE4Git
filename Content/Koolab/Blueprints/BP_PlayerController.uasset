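; Player controller that opens doors the player looks at and toggles every door with Space Bar.
; Each tick it traces from the pawn along the control rotation, opens an Anim_door hit within Distance and caches it as CurrAnim.
; A non-door or out-of-range hit closes the cached door; a trace with no hit leaves it as is.
; Space Bar flips IsDoorOpen and applies it to all Anim_door actors.
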(event `Key|SpaceBar`
  (params (Key :type "Key Structure"))
  ;[1 1 1] Open Or Close All Door
  (:`Pressed`
    (set `self.IsDoorOpen` (not (`self.IsDoorOpen`)))
    (bind _outactors (`GameplayStatics.GetAllActorsOfClass` "/Game/Koolab/Animation/Anim_door.Anim_door_C"))
    (for _array_element _outactors
      (`/Game/Koolab/Animation/Anim_door.SwitchDoor` _array_element (`self.IsDoorOpen`) false))))

(event `self.ReceiveTick`
  (params (DeltaSeconds :type "Float (single-precision)"))
  (bind _curranim (`self.CurrAnim`))
  (bind _returnvalue (`self.K2_GetActorLocation` (`self.K2_GetPawn`)))
  ;[1 1 1] Door auto open and close
  (bind _outhit (`KismetSystemLibrary.LineTraceSingleForObjects` _returnvalue (+ _returnvalue (* (`KismetMathLibrary.GetForwardVector` (`self.GetControlRotation`)) 10000.0)) (`|MakeArray` "ObjectTypeQuery1" "ObjectTypeQuery4" :!type "EObjectTypeQuery Enum")))
  (bind (_bblockinghit _binitialoverlap _time _distance _location _impactpoint _normal _impactnormal _physmat _hitactor) (`GameplayStatics.BreakHitResult` _outhit))
  (if _bblockinghit
    (if (<= (`KismetMathLibrary.VSize` (- _returnvalue (`self.K2_GetActorLocation` _hitactor))) (`self.Distance`))
      (bind _asanim_door (cast `/Game/Koolab/Animation/Anim_door` _hitactor)
        (:`then`
          (bind _output_get (set `self.CurrAnim` _asanim_door))
          (`/Game/Koolab/Animation/Anim_door.SwitchDoor` _output_get true false))
        (:`CastFailed`
          (`/Engine/EditorBlueprintResources/StandardMacros.IsValid` _curranim :!label _label
            (:`Is Valid`
              (`/Game/Koolab/Animation/Anim_door.SwitchDoor` _curranim false false)
              (set `self.CurrAnim` null)))))
      (else
        (goto _label)))))

(fn `UserConstructionScript`)